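; AI-controlled zombie character with faction membership, random navmesh wandering, projectile fire and health-based death.
; Perception updates filter actors by faction hostility and set EnemyActor through Neareast, though Hostiles is overwritten with one actor each time.
; Wander, attack-toggle and fire events have no callers here; wandering re-triggers itself on each successful move.
; Lethal damage detaches the controller and destroys the actor after a delay, while Tick drives walk speed.
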(event `FindRandomLocation`
  ;[1 1 1] prin
  (`|AIMoveTo` self (`NavigationSystem.K2_GetRandomLocationInNavigableRadius` (`self.K2_GetActorLocation` self) 2048.0)
    (:`OnSuccess`
      (`self.FindRandomLocation`))))

(event `self.ReceiveBeginPlay`)

(event `FactionAgentInterface.EventSetFaction`
  (params (Faction :type "Faction Structure (by ref)"))
  ;[0.8392 0.4654 0.2784 1 14] Faction Interfaces require GetFaction and SetFaction to work propertly
  (set `self.Faction` Faction))

(event `Enemy_Found`
  (set `self.EnableAttack` true))

(event `Enemy_Lost`
  (set `self.EnableAttack` false))

(event `self.AIPerception.OnPerceptionUpdated`
  (params (UpdatedActors :type "Array of Actor Object Reference (by ref)"))
  (if (== (`self.EnableDeath`) false)
    (for _array_element UpdatedActors
      (if (`FactionsLibrary.IsHostile` self _array_element)
        (bind _output_get (set `self.Hostiles` (`|MakeArray` _array_element)))
        (bind _closest (`self.Neareast` _output_get))
        (bind _output_get_2 (set `self.EnemyActor` _closest))
        (`KismetSystemLibrary.PrintString` (`KismetSystemLibrary.GetDisplayName` _output_get_2))))))

(event `FireAt`
  (`|SpawnActorFromClass` "/Game/ThirdPersonBP/Blueprints/Projecticle.Projecticle_C" (`SceneComponent.K2_GetComponentToWorld` (`self.Arrow1`)) "Undefined" "OverrideRootScale" self self)
  (`KismetSystemLibrary.PrintString` "fire"))

(event `self.ReceiveAnyDamage`
  (params (Damage :type "Float (single-precision)") (DamageType :type "DamageType Object Reference") (InstigatedBy :type "Controller Object Reference") (DamageCauser :type "Actor Object Reference"))
  (bind _health (`self.Health`))
  (if (<= _health 0.0)
    (`self.DetachFromControllerPendingDestroy` :!label _label)
    (set `self.EnableDeath` true)
    (`KismetSystemLibrary.PrintString` "im dead")
    (`KismetSystemLibrary.Delay` 10.0)
    (`self.K2_DestroyActor`)
    (else
      (bind _output_get (set `self.Health` (- _health Damage)))
      (if (<= _output_get 0.0)
        (goto _label)))))

(event `self.ReceiveTick`
  (params (DeltaSeconds :type "Float (single-precision)"))
  (set `CharacterMovementComponent.MaxWalkSpeed` (* (`self.SpeedRate`) (`self.speedVariable`)) (`self.CharacterMovement`)))

(fn `EventGetFaction`
  (returns (OutFaction :type "Faction Structure"))
  (return (`self.Faction`)))

(fn `Neareast`
  (params (Actors :type "Array of Actor Object Reference"))
  (returns (Closest :type "Actor Object Reference"))
  (for _array_element Actors
    (bind _returnvalue (`self.GetDistanceTo` _array_element self))
    (if (and (< _returnvalue (`self.ClosestDistance`)) (> _returnvalue (`self.MIN Distance`)))
      (set `self.Nearest` _array_element)
      (set `self.ClosestDistance` _returnvalue)
      (else
        (set `self.ClosestDistance` 10000000.0))))
  (return (`self.Nearest`)))

(fn `UserConstructionScript`)